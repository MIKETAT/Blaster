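; BP_BlasterCharacter is the Blaster character Blueprint, and its graph holds test and debug logic.
; On Tick, the authority auto-walks it forward and backward, using a Delay to flip MoveForward every couple of seconds as a self test.
; Holding the Tab debug key slows global time until release.
; An unconnected block would show the net role on the overhead widget for the locally controlled player only, but never runs.
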(event EventBeginPlay)

(event Collision|EventActorBeginOverlap
  (params (OtherActor :type Actor%20Object%20Reference)))

(event EventTick
  (params (DeltaSeconds :type Float%20%28single-precision%29))
  (bind _self self)
  (bind _returnvalue (Transformation|GetActorRotation _self))
  (bind _returnvalue_2 (Math|Vector|GetForwardVector _returnvalue))
  ;[1 1 1] self test
  (Networking|SwitchHasAuthority
    (:Authority
      (if (Variables|Default|GetMoveForward)
        (Pawn|Input|AddMovementInput _self _returnvalue_2 1.0 false)
        (Utilities|FlowControl|Delay 2.0)
        (Variables|Default|SetMoveForward false)
        (Development|PrintString "No Move Forward")
        (else
          (Pawn|Input|AddMovementInput _self _returnvalue_2 -1.0 false)
          (Utilities|FlowControl|Delay 2.0)
          (Variables|Default|SetMoveForward true)
          (Development|PrintString "Move Forward"))))))

(event Input|KeyboardEvents|DebugKeyTab
  (params (Key :type Key%20Structure :default "None") (ActionValue :type Input%20Action%20Value%20Structure))
  (:Pressed
    (Utilities|Time|SetGlobalTimeDilation 0.2))
  (:Released
    (Utilities|Time|SetGlobalTimeDilation 1.0)))

(fn ConstructionScript)